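; Zombie enemy that chases the player, attacks up close and takes damage until it dies.
; Tick re-issues AI MoveTo, gates a timed attack montage through DoOnce within melee range, and box-traces to apply damage on player hits.
; BeginPlay and Tick feed health to a ZHealth widget component.
; At zero health it ragdolls, destroys itself after a delay, and occasionally spawns one of two random actors.
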(event EventBeginPlay
  ;[1 1 1] Set Max Health
  (bind _aszhealth (Utilities|Casting|CastToZHealth (UserInterface|GetUserWidgetObject (Variables|Default|GetWidget))))
  (Variables|/Game/Blueprints/Zombie/ZHealth.ZHealth_C|SetMaxHealth _aszhealth (Variables|Default|GetHealth))
  (Variables|/Game/Blueprints/Zombie/ZHealth.ZHealth_C|SetHealth _aszhealth (Variables|Default|GetHealth)))

(event EventTick
  (params (DeltaSeconds :type Float%20%28single-precision%29))
  (bind _returnvalue (Game|GetPlayerCharacter 0))
  (bind _returnvalue_2 (Transformation|GetActorLocation _returnvalue))
  (Utilities|FlowControl|Sequence
    (:then_0
      ;[1 1 1] Makes Zombie Move to Player
      (AI|AIMoveTo self _returnvalue_2 _returnvalue 5.0 false
        (:then
          ;[1 1 1] Attacks if player gets too close
          (if (<= (Math|Vector|VectorLength (- _returnvalue_2 (Transformation|GetActorLocation))) 1.3e+02)
            (Utilities|FlowControl|DoOnce false
              (:Completed
                (bind _returnvalue_3 (Animation|PlayAnimMontage 0 1.0 "None"))
                (Utilities|FlowControl|Delay 0.6)
                (Variables|Default|SetAttacking true)
                (Utilities|FlowControl|Delay (- _returnvalue_3 0.6))
                (Variables|Default|SetAttacking false)))))))
    (:then_1
      ;[1 1 1] Checks if Zombie Hits Player
      (if true
        (for _array_element (Utilities|Array|MakeArray (Variables|Default|GetBox))
          (bind _outhit (Collision|BoxTraceByChannel (Transformation|GetWorldLocation _array_element) (Transformation|GetWorldLocation _array_element) (Components|Box|GetScaledBoxExtent _array_element) (Transformation|GetWorldRotation _array_element) "TraceTypeQuery1" false 0 "None"))
          (if (== (.HitActor (Collision|BreakHitResult _outhit)) (Game|GetPlayerCharacter 0))
            (Game|Damage|ApplyDamage 0 (Variables|Default|GetDamage) 0 0)))))
    (:then_2
      ;[1 1 1] Update Health bar
      (bind _aszhealth (Utilities|Casting|CastToZHealth (UserInterface|GetUserWidgetObject (Variables|Default|GetWidget))))
      (Variables|/Game/Blueprints/Zombie/ZHealth.ZHealth_C|SetHealth _aszhealth (Variables|Default|GetHealth))
      (Transformation|SetWorldRotation (Variables|Default|GetWidget) "180.000000,0.000000,0.000000" false false))))

(event Game|Damage|EventAnyDamage
  (params (Damage :type Float%20%28single-precision%29) (DamageType :type Damage%20Type%20Object%20Reference) (InstigatedBy :type Controller%20Object%20Reference) (DamageCauser :type Actor%20Object%20Reference))
  (bind _returnvalue (Transformation|GetActorTransform))
  ;[1 1 1] Ragdoll if Health <= 0
  (bind _output_get (Variables|Default|SetHealth (- (Variables|Default|GetHealth) Damage)))
  (if (<= _output_get 0.0)
    (Physics|SetSimulatePhysics (Variables|Character|GetMesh) true)
    (Collision|SetCollisionEnabled (Variables|Collision|GetCapsuleComponent) "NoCollision")
    (Utilities|FlowControl|Sequence
      (:then_0
        (Utilities|FlowControl|Delay 3.0)
        (Actor|DestroyActor))
      (:then_1
        (if (== (Math|Random|RandomIntegerinRange 0 9) 0)
          (Game|SpawnActorfromClass (Utilities|Select :Index (Math|Random|RandomIntegerinRange 0 1) :Option%200 0 :Option%201 0) (Math|Transform|MakeTransform (- (.location _returnvalue) "0.000000,0.000000,60.000000") (.rotation _returnvalue) (.scale _returnvalue)) "Undefined" 0))))))

(fn ConstructionScript)