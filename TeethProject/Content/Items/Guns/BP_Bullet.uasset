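; BP_Bullet is a gun projectile that damages zombies on hit.
; On BeginPlay it copies its Velocity variable into the ProjectileMovement component.
; Its Sphere overlap reacts only to the Box component of a BP_Zombie, then destroys the bullet, plays hitmarker and zombie death 2D sounds, and applies fixed damage.
; The death sound plays on every qualifying hit, and damage is applied after the DestroyActor call.
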(event OnComponentBeginOverlap(Sphere)
  (params (OverlappedComponent :type Primitive%20Component%20Object%20Reference) (OtherActor :type Actor%20Object%20Reference) (OtherComp :type Primitive%20Component%20Object%20Reference) (OtherBodyIndex :type Integer) (bFromSweep :type Boolean) (SweepResult :type Hit%20Result%20Structure%20%28by%20ref%29))
  (bind _asbp_zombie (Utilities|Casting|CastToBP_Zombie OtherActor))
  (if (== OtherComp (Variables|/Game/Enemies/Blueprints/BP_Zombie.BP_Zombie_C|GetBox _asbp_zombie))
    (Utilities|FlowControl|Sequence
      (:then_0
        (Actor|DestroyActor)
        (Audio|PlaySound2D "/Game/Assets/Audio/Hitmarker.Hitmarker" 0.5 1.0 0.0 0 0)
        (Audio|PlaySound2D "/Game/Assets/Audio/zombie_death.zombie_death" 0.6 1.0 0.0 0 0))
      (:then_1
        (Game|Damage|ApplyDamage _asbp_zombie 0.25 0 0)))))

(event EventBeginPlay
  (Variables|/Script/Engine.MovementComponent|SetVelocity (Variables|Default|GetProjectileMovement) (Variables|Default|GetVelocity)))

(fn ConstructionScript)