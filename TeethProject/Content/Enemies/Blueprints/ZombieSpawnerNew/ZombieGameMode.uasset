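; Game mode for a round-based zombie mode that starts the first round on BeginPlay.
; IncreaseRound bumps the round number, waits briefly, then StartRound sets the zombie total, fixed for round one and scaled from MaxZombies afterwards.
; A looping timer calls Spawn on the first BP_ZombieSpawner found until that total is reached, then clears itself.
; Nothing here advances later rounds or resets the spawned count.
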(event Custom|IncreaseRound
  (Math|Integer|IncrementInt (Variables|Default|GetRoundNumber)
    (:%20%20
      (Utilities|FlowControl|Delay 5.0)
      (CallFunction|StartRound))))

(event Custom|SpawnZombie
  (if (< (Variables|Default|GetZombiesSpawned) (Variables|Default|GetTotalZombiesInRound))
    (bind _outactors (Actor|GetAllActorsOfClass "/Game/Enemies/Blueprints/ZombieSpawnerNew/BP_ZombieSpawner.BP_ZombieSpawner_C"))
    (Default|Spawn (Utilities|Array|Get(acopy) _outactors) 0.0)
    (Math|Integer|IncrementInt (Variables|Default|GetZombiesSpawned))
    (else
      (Utilities|Time|ClearandInvalidateTimerbyHandle (stale Custom|StartRound _returnvalue)))))

(event Custom|StartRound
  (Variables|Default|SetTotalZombiesInRound (select (== (Variables|Default|GetRoundNumber) 1) 6 (Math|Float|Round (* (* (Variables|Default|GetRoundNumber) 0.15) (Variables|Default|GetMaxZombies)))))
  (bind _returnvalue (Utilities|Time|SetTimerbyEvent (delegate Custom|SpawnZombie) (Variables|Default|GettimeBetweenEachSpawn) true)))

(event EventBeginPlay
  (CallFunction|IncreaseRound))

(event EventTick
  (params (DeltaSeconds :type Float%20%28single-precision%29)))

(fn ConstructionScript)