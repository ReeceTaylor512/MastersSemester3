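; Zombie enemy that chases and melee-attacks the player, registering itself in the game mode's living-enemy count.
; Tick drives AIMoveTo, refreshes the health bar widget, and damages the player every frame the hit box overlaps during the montage-timed attack window.
; AnyDamage lowers health; at zero the mesh ragdolls, the game mode is notified, a random chance spawns one of two actors, and the zombie is destroyed after a delay.
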(event EventBeginPlay
  (Utilities|FlowControl|Sequence
    (:then_0
      (bind _asbp_first_person_game_mode (Utilities|Casting|CastToBP_FirstPersonGameMode (Game|GetGameMode)))
      (Math|Integer|IncrementInt (Variables|/Game/Player/BP_FirstPersonGameMode.BP_FirstPersonGameMode_C|GetEnemyAlive _asbp_first_person_game_mode)))
    (:then_1
      ;[1 1 1] Set MaxHealth
      (bind _aszhealth (Utilities|Casting|CastToZHealth (UserInterface|GetUserWidgetObject (Variables|Default|GetWidget))))
      (Variables|/Game/Enemies/Blueprints/ZHealth.ZHealth_C|SetMaxHealth _aszhealth (Variables|Default|GetHealth))
      (Variables|/Game/Enemies/Blueprints/ZHealth.ZHealth_C|SetHealth _aszhealth (Variables|Default|GetHealth)))))

(event Collision|EventActorBeginOverlap
  (params (OtherActor :type Actor%20Object%20Reference)))

(event EventTick
  (params (DeltaSeconds :type Float%20%28single-precision%29))
  (bind _returnvalue (Game|GetPlayerCharacter 0))
  (bind _box (Variables|Default|GetBox))
  (bind _returnvalue_2 (Collision|IsOverlappingActor _box _returnvalue :!class /Script/Engine.PrimitiveComponent))
  (bind _asue_4asp_character (Utilities|Casting|CastToUe4ASP_Character _returnvalue))
  (Utilities|FlowControl|Sequence
    (:then_0
      ;[1 1 1] Makes the zombie move to the player character
      (AI|AIMoveTo self "0, 0, 0" _returnvalue 5.0 false
        (:then
          ;[1 1 1] Attacks if close enough to player
          (if _returnvalue_2
            (Utilities|FlowControl|DoOnce false :!label _label
              (:Completed
                (bind _returnvalue_3 (Animation|PlayAnimMontage 0 1.0 "None"))
                (Utilities|FlowControl|Delay 0.6)
                (Variables|Default|SetAttacking true)
                (Utilities|FlowControl|Delay (- _returnvalue_3 0.6))
                (Variables|Default|SetAttacking false)
                (goto _label Reset)))))))
    (:then_1
      ;[1 1 1] UpdateHealthBar
      (bind _aszhealth (Utilities|Casting|CastToZHealth (UserInterface|GetUserWidgetObject (Variables|Default|GetWidget))))
      (Variables|/Game/Enemies/Blueprints/ZHealth.ZHealth_C|SetHealth _aszhealth (Variables|Default|GetHealth))
      (Transformation|SetWorldRotation (Variables|Default|GetWidget) "180.000000,0.000000,0.000000" false false))
    (:then_2
      ;[1 1 1] Checks if zombie hits player
      (if (and _returnvalue_2 (Variables|Default|GetAttacking))
        (Development|PrintString "attack")
        ;;[1 1 1] Damages the player
        (Default|DamagePlayer _asue_4asp_character (- (Variables|/Game/Player/AnimStarterPack/Ue4ASP_Character.Ue4ASP_Character_C|GetHealth _asue_4asp_character) (Variables|Default|GetDamage)))))))

(event Game|Damage|EventAnyDamage
  (params (Damage :type Float%20%28single-precision%29) (DamageType :type Damage%20Type%20Object%20Reference) (InstigatedBy :type Controller%20Object%20Reference) (DamageCauser :type Actor%20Object%20Reference))
  (bind _returnvalue (Transformation|GetActorTransform))
  ;[1 1 1] Ragdoll if health lessthen/equal 0
  (bind _output_get (Variables|Default|SetHealth (- (Variables|Default|GetHealth) Damage)))
  (if (<= _output_get 0.0)
    (Physics|SetSimulatePhysics (Variables|Character|GetMesh) true)
    (Collision|SetCollisionEnabled (Variables|Collision|GetCapsuleComponent) "NoCollision")
    (Utilities|FlowControl|Sequence
      (:then_0
        (bind _asbp_first_person_game_mode (Utilities|Casting|CastToBP_FirstPersonGameMode (Game|GetGameMode)))
        (Math|Integer|DecrementInt (Variables|/Game/Player/BP_FirstPersonGameMode.BP_FirstPersonGameMode_C|GetEnemyAlive _asbp_first_person_game_mode)
          (:%20%20
            (Default|RemainingEnemies _asbp_first_person_game_mode)
            (Utilities|FlowControl|Delay 3.0)
            (Actor|DestroyActor))))
      (:then_1
        (if (== (Math|Random|RandomIntegerinRange 0 8) 0)
          (Game|SpawnActorfromClass (Utilities|Select :Index (Math|Random|RandomIntegerinRange 0 1) :Option%200 0 :Option%201 0) (Math|Transform|MakeTransform (- (.location _returnvalue) "0, 0,60.000000") (.rotation _returnvalue) (.scale _returnvalue)) "Undefined" 0 0))))))

(fn ConstructionScript)