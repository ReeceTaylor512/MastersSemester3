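; Actor that spawns zombies in waves, with a per-wave count read from the ZombiesSpawned array.
; CheckForWaveEnd runs on BeginPlay, waits briefly, then proceeds only if an actor-class query returns nothing and the wave index is valid.
; Each zombie spawns at a random SpawnLocation offset from the spawner, then WaveNo increments.
; The check does not reschedule itself, so later waves need another call to CheckForWaveEnd.
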(event Custom|CheckForWaveEnd
  (bind _zombiesspawned (Variables|Default|GetZombiesSpawned))
  (bind _waveno (Variables|Default|GetWaveNo))
  (bind _spawnlocation (Variables|Default|GetSpawnLocation))
  (Utilities|FlowControl|Delay 0.2)
  (bind _outactors (Actor|GetAllActorsOfClass 0))
  (if (== (Utilities|Array|Length _outactors) 0)
    (if (Utilities|Array|IsValidIndex _zombiesspawned _waveno)
      (for _index (range 1 (Utilities|Array|Get(acopy) _zombiesspawned _waveno))
        (Game|SpawnActorfromClass "/Game/Blueprints/Zombie/Zombie.Zombie_C" (Math|Transform|MakeTransform (+ (Utilities|Array|Get(acopy) _spawnlocation (Math|Random|RandomIntegerinRange 0 (Utilities|Array|LastIndex _spawnlocation))) (Transformation|GetActorLocation)) "0, 0, 0" "1.000000,1.000000,1.000000") "Undefined" 0 0))
      (Math|Integer|IncrementInt (Variables|Default|GetWaveNo)))))

(event EventBeginPlay
  (CallFunction|CheckforWaveEnd))

(fn ConstructionScript)