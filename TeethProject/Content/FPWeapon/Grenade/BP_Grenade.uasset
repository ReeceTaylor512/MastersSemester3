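; BP_Grenade is a projectile grenade that explodes when its static mesh hits something.
; The construction script sets the projectile movement's initial speed from the Impulse variable.
; On hit, it plays a sound, spawns a scaled-up particle effect and applies radial damage at the hit's trace end.
; Delays then remove the effect and destroy the actor; the GrenadeData function is empty.
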(event OnComponentHit(StaticMesh)
  (params (HitComponent :type Primitive%20Component%20Object%20Reference) (OtherActor :type Actor%20Object%20Reference) (OtherComp :type Primitive%20Component%20Object%20Reference) (NormalImpulse :type Vector :default "0, 0, 0") (Hit :type Hit%20Result%20Structure%20%28by%20ref%29))
  (bind _traceend (Collision|BreakHitResult Hit))
  (Audio|PlaySoundatLocation "/Game/FPWeapon/Grenade/Sound/Explosion.Explosion" _traceend "0, 0, 0" 1.0 1.0 0.0 0 0 0 0)
  (bind _returnvalue (Effects|SpawnEmitteratLocation "/Game/FPWeapon/Grenade/Emitter/Explosion.Explosion" _traceend "0, 0, 0" "50.000000,50.000000,50.000000"))
  (Game|Damage|ApplyRadialDamage 1e+02 _traceend 7e+02 "/Script/Engine.DamageType" 0 0 0 false "ECC_Visibility")
  (Utilities|FlowControl|Delay 1.0) ; Timer destroy particle effect
  (Components|DestroyComponent _returnvalue)
  (Utilities|FlowControl|Delay 0.2) ; Time to destroy the mesh
  (Actor|DestroyActor))

(fn ConstructionScript
  (Variables|/Script/Engine.ProjectileMovementComponent|SetInitialSpeed (Variables|Default|GetProjectileMovement) (Variables|Default|GetImpulse)))

(fn GrenadeData)